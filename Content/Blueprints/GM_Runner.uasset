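; GM_Runner, apparently the game mode for a multiplayer race, handles the start, winner announcement and level restart.
; BeginPlay waits out a countdown, prints the start message and calls the StartRace dispatcher.
; AnnounceWinner uses IsRaceOver to accept only the first winner, prints their index, calls AnnouncedWinner and starts a five-second one-shot timer.
; RestartLevel reopens the current level by name, likely as that timer's callback.
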(event EventBeginPlay
  (Utilities|FlowControl|Delay (Variables|Default|GetCountDown))
  (Development|PrintString "Race Start")
  (Default|CallStartRace))

(event EventTick
  (params (DeltaSeconds :type Float%20%28single-precision%29)))

(fn ConstructionScript)

(fn AnnounceWinner
  (params (WinnerIndex :type Integer))
  (if (not (Variables|Default|GetIsRaceOver))
    (Variables|Default|SetIsRaceOver true)
    (Development|PrintString (Utilities|String|Append "Player" (Utilities|String|ToString(Integer) WinnerIndex) "IS THE WINNER!!!"))
    (Default|CallAnnouncedWinner)
    (Utilities|Time|SetTimerbyEvent (EventDispatchers|CreateEvent :!event RestartLevel) 5.0)))

(fn RestartLevel
  (bind _returnvalue (Game|GetCurrentLevelName true))
  (Game|OpenLevel(byName) (Utilities|String|StringToName _returnvalue)))